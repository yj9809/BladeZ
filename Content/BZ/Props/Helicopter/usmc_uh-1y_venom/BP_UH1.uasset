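; BP_UH1 is a UH-1Y Venom helicopter prop that plays audio on start and eases toward a TargetLocation.
; Tick spins the main rotor from RotorRPM and the tail rotor at a fixed multiple of that speed.
; Beyond a small radius of the target, sine and Perlin noise add bob and sway.
; Within it, a second interpolation settles position and eases rotation toward zero.
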(event EventBeginPlay
  (Audio|Components|Audio|Play (Variables|Default|GetAudio) 0.0))

(event EventTick
  (params (DeltaSeconds :type Float%20%28single-precision%29))
  (bind _returnvalue (Transformation|GetActorLocation))
  (bind _returnvalue_2 (Utilities|Time|GetGameTimeinSeconds))
  (bind _rotorrpm (Variables|Default|GetRotorRPM))
  (bind _targetlocation (Variables|Default|GetTargetLocation))
  (bind _returnvalue_3 (* DeltaSeconds _rotorrpm -6.0))
  (bind _returnvalue_4 (* _returnvalue_2 2.0))
  (Transformation|AddLocalRotation (Variables|Default|GetMainRotor) (Math|Rotator|MakeRotator 0.0 0.0 _returnvalue_3) false false)
  (Transformation|AddLocalRotation (Variables|Default|GetTailRotor) (Math|Rotator|MakeRotator (* _returnvalue_3 5.56) 0.0 0.0) false false)
  (Transformation|SetActorLocation (Math|Interpolation|VInterpTo (Transformation|GetActorLocation) (Variables|Default|GetTargetLocation) DeltaSeconds 0.5) false false)
  (if (Utilities|Operators|EqualEqual _returnvalue _targetlocation 3e+01)
    (Transformation|SetActorLocationAndRotation (Math|Interpolation|VInterpTo _returnvalue _targetlocation DeltaSeconds 1.0) (Math|Interpolation|RInterpTo (Transformation|GetActorRotation) "0, 0, 0" DeltaSeconds 1.0))
    (else
      (Class|Actor|AddActorLocalTransform (Math|Transform|MakeTransform (Math|Vector|MakeVector 0.0 0.0 (+ (* (Math|Trig|Sin(Radians) _returnvalue_4) 0.3) (* (Class|KismetMathLibrary|PerlinNoise1D _returnvalue_4) 0.5))) (Math|Rotator|MakeRotator (+ 0.0 (* (Class|KismetMathLibrary|PerlinNoise1D (* (+ _returnvalue_2 2.0) 1.0)) 0.2)) (+ 0.0 (* (Class|KismetMathLibrary|PerlinNoise1D (* (+ _returnvalue_2 3.2) 1.0)) 0.2)) 0.0) (Transformation|GetActorScale3D)) false false))))

(fn ConstructionScript)