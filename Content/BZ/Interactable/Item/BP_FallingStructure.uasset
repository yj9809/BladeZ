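; BP_FallingStructure is a destructible structure that collapses when the player enters its activation trigger.
; The overlap calls TriggerCollapse, enables Geometry Collection physics, then applies external strain and radial impulses at left, center and right points.
; All three branches share a delay that later stops physics simulation and sets a lifespan for cleanup.
; Geometry Collection hits on zombies call ExecuteRadialCrush at the impact location.
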(event OnComponentBeginOverlap(ActivationTrigger)
  (params (OverlappedComponent :type Primitive%20Component%20Object%20Reference) (OtherActor :type Actor%20Object%20Reference) (OtherComp :type Primitive%20Component%20Object%20Reference) (OtherBodyIndex :type Integer) (bFromSweep :type Boolean) (SweepResult :type Hit%20Result%20Structure%20%28by%20ref%29))
  (bind _geometrycollection (Variables|Default|GetGeometryCollection))
  (bind _fieldposition_left (Variables|Default|GetFieldPosition_Left))
  (bind _fieldposition_center (Variables|Default|GetFieldPosition_Center))
  (bind _fieldposition_right (Variables|Default|GetFieldPosition_Right))
  (bind _returnvalue (Transformation|GetWorldLocation _fieldposition_right))
  (bind _returnvalue_2 (Transformation|GetWorldLocation _fieldposition_left))
  (bind _returnvalue_3 (Transformation|GetWorldLocation _fieldposition_center))
  (Utilities|Casting|CastToBZPlayerCharacter OtherActor)
  (Class|BZFallingStructure|TriggerCollapse)
  (Physics|SetSimulatePhysics _geometrycollection true)
  (Utilities|FlowControl|Sequence
    (:then_0
      (Class|GeometryCollectionComponent|ApplyExternalStrain _geometrycollection 0 _returnvalue_2 8e+02 0 1.0 5e+10)
      (Class|PhysicsObjectBlueprintLibrary|ApplyRadialImpulse _geometrycollection _returnvalue_2 1.2e+03 1e+05 "RIF_Constant" true 0.0 false 0.0 1.0))
    (:then_1
      (Class|GeometryCollectionComponent|ApplyExternalStrain _geometrycollection 0 _returnvalue_3 8e+02 0 1.0 5e+07)
      (Class|PhysicsObjectBlueprintLibrary|ApplyRadialImpulse _geometrycollection _returnvalue_3 1.2e+03 1e+04 "RIF_Constant" true 0.0 false 0.0 1.0))
    (:then_2
      (Class|GeometryCollectionComponent|ApplyExternalStrain _geometrycollection 0 _returnvalue 8e+02 0 1.0 5e+08)
      (Class|PhysicsObjectBlueprintLibrary|ApplyRadialImpulse _geometrycollection _returnvalue 1.2e+03 1e+05 "RIF_Constant" true 0.0 false 0.0 1.0)))
  (Utilities|FlowControl|Delay 3.0)
  (Physics|SetSimulatePhysics (Variables|Default|GetGeometryCollection) false)
  (Actor|SetLifeSpan 4.0))

(event OnComponentHit(GeometryCollection)
  (params (HitComponent :type Primitive%20Component%20Object%20Reference) (OtherActor :type Actor%20Object%20Reference) (OtherComp :type Primitive%20Component%20Object%20Reference) (NormalImpulse :type Vector :default "0, 0, 0") (Hit :type Hit%20Result%20Structure%20%28by%20ref%29))
  (Utilities|IsValid OtherActor
    (:Is%20Valid
      (Utilities|Casting|CastToBZZombie OtherActor)
      (Class|BZFallingStructure|ExecuteRadialCrush (.Location (Collision|BreakHitResult Hit))))))

(fn ConstructionScript)