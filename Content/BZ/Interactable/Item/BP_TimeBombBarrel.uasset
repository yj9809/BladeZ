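; BP_TimeBombBarrel is an interactable barrel item that detonates after a pulsing fuse when destroyed.
; On destruction, a timeline's Pulse track drives the mesh's glow and scale as a warning.
; When the timeline finishes, it spawns a Niagara fire effect and applies radial damage, ignoring itself.
; After a short delay it draws a debug sphere of the blast radius and calls ExplodeAndDropItem.
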(event EventOnItemDestroyed
  (params (InstigatorPawn :type Actor%20Object%20Reference))
  (bind _returnvalue (Transformation|GetActorLocation))
  (bind _self self)
  (bind _itemmesh (Variables|Default|GetItemMesh))
  (bind _pulse (Timeline|ExplosionTimeline PlayFromStart)
    (:Update
      (Rendering|Material|SetScalarParameterValueonMaterials _itemmesh "GlowIntensity" _pulse)
      (Transformation|SetRelativeScale3D _itemmesh (Math|Conversions|ToVector(Float) (Math|Float|Lerp 1.1 1.2 _pulse))))
    (:Finished
      (Niagara|SpawnSystematLocation "/Game/AdvancedMagicFX12/particles/Niagara/NS_ky_hit_fire.NS_ky_hit_fire" _returnvalue)
      (Game|Damage|ApplyRadialDamage 1e+01 _returnvalue 4e+02 "/Script/Engine.DamageType" (Utilities|Array|MakeArray _self) _self 0 false "ECC_Visibility")
      (Utilities|FlowControl|Delay 0.5)
      (Rendering|Debug|DrawDebugSphere _returnvalue 4e+02 24 "(R=1.000000,G=0.000000,B=0.000000,A=1.000000)" 2.0 2.0)
      (Class|BZInteractItemBase|ExplodeandDropItem))))

(fn ConstructionScript)