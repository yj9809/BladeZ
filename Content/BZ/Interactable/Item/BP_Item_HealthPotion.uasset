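; BP_Item_HealthPotion is an interactable item that heals the player when its item effect is applied.
; It overrides ApplyItemEffect, calls the parent, then heals by passing negative damage to ApplyDamage on the player, printing the returned value.
; It then spawns the NS_Prestige_Slash_Impact effect, calls PlaySoundAtLocation with no sound asset shown, and destroys itself.
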(fn ConstructionScript
  (|CallParentFunction))

(fn ApplyItemEffect
  (params (Player :type BZ%20Player%20Character%20Object%20Reference))
  (bind _returnvalue (Transformation|GetActorLocation))
  (|CallParentFunction Player)
  (bind _returnvalue_2 (Game|Damage|ApplyDamage Player -5e+01 0 self "/Script/Engine.DamageType"))
  (Development|PrintString (Utilities|String|ToString(Float) _returnvalue_2))
  (Niagara|SpawnSystematLocation "/Game/Hack_And_Slash_FX/VFX_Niagara/Impacts/NS_Prestige_Slash_Impact.NS_Prestige_Slash_Impact" _returnvalue)
  (Audio|PlaySoundatLocation 0 _returnvalue "0, 0, 0" 1.0 1.0 0.0 0 0 0 0)
  (Actor|DestroyActor))