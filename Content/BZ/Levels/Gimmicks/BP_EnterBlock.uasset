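; BP_EnterBlock is a level gimmick that seals an entrance after something enters its Detect volume.
; The first overlap, with no actor filter, sets a one-shot flag, enables Block collision, calls CallPlaySequence and hides the StaticMesh a second later.
; A separate BlockEntrance_Event, with no caller in this graph, teleports the mesh to BlockTransform and makes it visible again.
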(event OnComponentBeginOverlap(Detect)
  (params (OverlappedComponent :type Primitive%20Component%20Object%20Reference) (OtherActor :type Actor%20Object%20Reference) (OtherComp :type Primitive%20Component%20Object%20Reference) (OtherBodyIndex :type Integer) (bFromSweep :type Boolean) (SweepResult :type Hit%20Result%20Structure%20%28by%20ref%29))
  (if (not (Variables|Default|GetbIsStarted))
    (Variables|Default|SetbIsStarted true)
    (Collision|SetCollisionEnabled (Variables|Default|GetBlock) "QueryAndPhysics")
    (Default|CallPlaySequence)
    (Utilities|FlowControl|Delay 1.0)
    (Rendering|SetVisibility (Variables|Default|GetStaticMesh) false false)))

(event Custom|BlockEntrance_Event
  (bind _blocktransform (Variables|Default|GetBlockTransform))
  (Transformation|SetWorldLocationAndRotation (Variables|Default|GetStaticMesh) (.location _blocktransform) (.rotation _blocktransform) false true)
  (Rendering|SetVisibility (Variables|Default|GetStaticMesh) true false))

(event EventBeginPlay)

(event Collision|EventActorBeginOverlap
  (params (OtherActor :type Actor%20Object%20Reference)))

(event EventTick
  (params (DeltaSeconds :type Float%20%28single-precision%29)))

(fn ConstructionScript)