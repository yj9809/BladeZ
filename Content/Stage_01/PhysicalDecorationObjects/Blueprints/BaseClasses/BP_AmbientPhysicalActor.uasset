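; Base actor for ambient physical decoration props that play impact sounds and can break.
; On hit, fast breakable props striking non-simulating components call the empty Break function once; otherwise sufficiently fast hits play sound, with volume from speed and pitch from scale.
; HitByTrace triggers the same break, bypassing those checks.
; Construction sets mesh, optional replication and a shared dynamic material with custom or seeded-random tint and optional random UV offset.
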(event Custom|PlayCollisionSounds
  ;[1 1 1] play the collision sound
  ;;[1 1 1] Rules when and how loud to play the sound based on objects velocity
  (bind _returnvalue (Physics|GetPhysicsLinearVelocity (Variables|Default|GetStaticMeshComponent) "None"))
  ;;[1 1 1] finally play the sound
  (Audio|PlaySoundatLocation (Variables|Assets|GetCollisionSound) (Variables|DestructionRelated|GetWorldHitLocation) "0, 0, 0" (Math|Float|MapRangeClamped (Math|Vector|VectorLength _returnvalue) 0.0 (Variables|VolumeIncreaseAtHighImpactSpeeds|GetMaxSpeedToVolume) (Variables|VolumeIncreaseAtHighImpactSpeeds|GetMinVolume) (Variables|VolumeIncreaseAtHighImpactSpeeds|GetMaxVolume)) (Math|Float|MapRangeClamped (Math|Float|Absolute(Float) (.X (Math|Vector|BreakVector (Transformation|GetActorScale3D self)))) 1.0 3.0 1.0 (Variables|PitchDecreaseWithHigherObjectScale|GetMinimumPitchAtScale)) 0.0 0 0 0 0))

(event Custom|HitByTrace
  ;[1 1 1] conditions to break object and finally break
  (Utilities|FlowControl|DoOnce false
    (:Completed
      (CallFunction|Break))))

(event Collision|EventHit
  (params (MyComp :type Primitive%20Component%20Object%20Reference) (Other :type Actor%20Object%20Reference) (OtherComp :type Primitive%20Component%20Object%20Reference) (bSelfMoved :type Boolean) (HitLocation :type Vector :default "0, 0, 0") (HitNormal :type Vector :default "0, 0, 0") (NormalImpulse :type Vector :default "0, 0, 0") (Hit :type Hit%20Result%20Structure%20%28by%20ref%29))
  (Utilities|FlowControl|Sequence
    (:then_0
      ;[1 1 1] set impact  prequisites
      (Variables|DestructionRelated|SetWorldHitLocation HitLocation)
      (Variables|DestructionRelated|SetImpulseVector NormalImpulse)
      (bind _output_get (Variables|Default|SetOtherComp OtherComp))
      (Variables|DestructionRelated|SetHitCompIsPhysical (Physics|IsSimulatingPhysics _output_get "None")))
    (:then_1
      ;[1 1 1] conditions to break object and finally break
      (Utilities|IsValid (Variables|Default|GetStaticMeshComponent)
        (:Is%20Valid
          (bind _returnvalue (Physics|GetPhysicsLinearVelocity (Variables|Default|GetStaticMeshComponent) "None"))
          (if (and (> (Math|Vector|VectorLength _returnvalue) (Variables|DestructionRelated|GetSpeedToBreakObject)) (and (Variables|DestructionRelated|GetObjectIsBreakable) (not (Variables|DestructionRelated|GetHitCompIsPhysical))))
            (Utilities|FlowControl|DoOnce false
              (:Completed
                (CallFunction|Break)))
            (else
              ;[1 1 1] Is the object moving fast enough to make a sound?
              (if (> (Math|Vector|VectorLength (Transformation|GetComponentVelocity (Variables|Default|GetStaticMeshComponent))) (Variables|SoundInitiator|GetMinimumSpeedToSound))
                (CallFunction|PlayCollisionSounds)))))))))

(fn ConstructionScript
  (bind _self self)
  (bind _staticmeshcomponent (Variables|Default|GetStaticMeshComponent))
  (bind _syncronizeovernet (Variables|Assets|GetSyncronizeOverNet))
  ;[1 1 1] set mesh and network replication
  (Components|StaticMesh|SetStaticMesh _staticmeshcomponent (Variables|Assets|GetStaticMesh))
  (Class|ActorComponent|SetIsReplicated _staticmeshcomponent _syncronizeovernet)
  (Networking|SetReplicates _self _syncronizeovernet)
  (Class|Actor|SetReplicateMovement _self _syncronizeovernet)
  (Audio|Components|Audio|SetSound (Variables|Default|GetPhysicalSoundComponent) (Variables|Assets|GetCollisionSound))
  ;[1 1 1] create a random stream and the dynamic material
  (Variables|ColorTintAndUVs|SetRandomStream (Math|Random|MakeRandomStream (Variables|ColorTintAndUVs|GetRandomSeed)))
  (bind _returnvalue (Rendering|Material|CreateDynamicMaterialInstance (Variables|Default|GetStaticMeshComponent) 0 (Variables|Assets|GetMaterialSource) "None" :!class /Script/Engine.PrimitiveComponent))
  (Variables|Assets|SetDynamicMaterial _returnvalue)
  ;[1 1 1] set all static meshes to have the dynamic material and also set a possible LOD material
  (for _array_element (Actor|GetComponentsByClass self "/Script/Engine.StaticMeshComponent")
    (if (== (Utilities|Array|Length (Rendering|Material|GetMaterials _array_element)) 2)
      (Rendering|Material|SetMaterial _array_element 0 (Variables|Assets|GetDynamicMaterial))
      (Rendering|Material|SetMaterial _array_element 1 (Variables|Assets|GetDynamicMaterial))
      (else
        (Rendering|Material|SetMaterial _array_element 0 (Variables|Assets|GetDynamicMaterial))))
    (if (Variables|ColorTintAndUVs|GetRandomizeTinting)
      ;[1 1 1] Randomizing
      (Utilities|FlowControl|Sequence
        (:then_0
          ;;[1 1 1] Material Tinting
          (Rendering|Material|SetVectorParameterValue (Variables|Assets|GetDynamicMaterial) "TintColor" (Class|KismetMathLibrary|HSVtoRGB (Math|Random|RandomFloatinRangefromStream (Variables|ColorTintAndUVs|GetRandomStream) 0.0 3.6e+02) (Math|Random|RandomFloatinRangefromStream (Variables|ColorTintAndUVs|GetRandomStream) 0.0 1.0) (Math|Random|RandomFloatinRangefromStream (Variables|ColorTintAndUVs|GetRandomStream) 0.0 1.0) 1.0) :!class /Script/Engine.MaterialInstanceDynamic))
        (:then_1
          (Rendering|Material|SetScalarParameterValue (Variables|Assets|GetDynamicMaterial) "TintIntensity" (Variables|ColorTintAndUVs|GetTintIntensity) :!class /Script/Engine.MaterialInstanceDynamic))
        (:then_2
          ;;[1 1 1] MoveUVs
          (if (Variables|ColorTintAndUVs|GetMoveTileableUVsRandomly) :!label _label
            (Rendering|Material|SetScalarParameterValue (Variables|Assets|GetDynamicMaterial) "UV_Paning" (Math|Random|RandomFloat) :!class /Script/Engine.MaterialInstanceDynamic))))
      (else
        ;[1 1 1] Customize
        (Utilities|FlowControl|Sequence
          (:then_0
            ;;[1 1 1] Material Tinting
            (Rendering|Material|SetVectorParameterValue (Variables|Assets|GetDynamicMaterial) "TintColor" (Variables|ColorTintAndUVs|GetTintColor) :!class /Script/Engine.MaterialInstanceDynamic))
          (:then_1
            (Rendering|Material|SetScalarParameterValue (Variables|Assets|GetDynamicMaterial) "TintIntensity" (Variables|ColorTintAndUVs|GetTintIntensity) :!class /Script/Engine.MaterialInstanceDynamic))
          (:then_2
            (goto _label)))))))

(fn Break)