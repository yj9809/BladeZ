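; BP_TileTool is a construction-script tool that lays out one mesh, or optionally two, in a width-by-depth grid.
; Each mesh runs through the shared Tile function, which creates a hierarchical instanced static mesh component and adds the grid instances.
; Spacing comes from the mesh's local bounds or a width/depth override, with per-mesh offset, yaw and reversible X/Y direction.
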(event EventBeginPlay)

(event Collision|EventActorBeginOverlap
  (params (OtherActor :type Actor%20Object%20Reference)))

(event EventTick
  (params (DeltaSeconds :type Float%20%28single-precision%29)))

(fn ConstructionScript
  (bind _tile_01_offset (Variables|TileMesh01|GetTile%2001%20Offset))
  (bind _tile_02_offset (Variables|TileMesh02|GetTile%2002%20Offset))
  (CallFunction|Tile (Variables|TileMesh01|GetTileMesh_01) (Variables|TileMesh01|GetOverride%20Tile%2001%20Width) (Variables|TileMesh01|GetOverride%20Tile%2001%20Depth) (.x _tile_01_offset) (.y _tile_01_offset) (.z _tile_01_offset) (Variables|TileMesh01|GetTile%2001%20Rotation) (Variables|TileMesh01|GetUse%20Min%20X%20as%20Tile%2001%20Bound?) (Variables|TileMesh01|GetUse%20Min%20Y%20as%20Tile%2001%20Bound?) (Variables|TileMesh01|GetOverrideTile01Width?) (Variables|TileMesh01|GetOverrideTile01Depth?) (Variables|TileMesh01|GetReverseTile01X?) (Variables|TileMesh01|GetReverseTile01Y?))
  (if (Variables|TileMesh02|GetAdd%20Tile%20Mesh%2002?)
    (CallFunction|Tile (Variables|TileMesh02|GetTileMesh_02) (Variables|TileMesh02|GetOverride%20Tile%2002%20Width) (Variables|TileMesh02|GetOverride%20Tile%2002%20Depth) (.x _tile_02_offset) (.y _tile_02_offset) (.z _tile_02_offset) (Variables|TileMesh02|GetTile%2002%20Rotation) (Variables|TileMesh02|GetUse%20Min%20X%20as%20Tile%2002%20Bound?) (Variables|TileMesh02|GetUse%20Min%20Y%20as%20Tile%2002%20Bound?) (Variables|TileMesh02|GetOverrideTile02Width?) (Variables|TileMesh02|GetOverrideTile02Depth?) (Variables|TileMesh02|GetReverseTile02X?) (Variables|TileMesh02|GetReverseTile02Y?))))

(fn Tile
  (params (Tile%20Mesh%2001 :type Static%20Mesh%20Object%20Reference) (Override%20Tile%20Width :type Float%20%28double-precision%29) (Override%20Tile%20Depth :type Float%20%28double-precision%29) (X%20Offset :type Float%20%28double-precision%29) (Y%20Offset :type Float%20%28double-precision%29) (Z%20Offset :type Float%20%28double-precision%29) (Rotation :type Float%20%28double-precision%29) (UseMinXBound :type Boolean) (UseMinYBound :type Boolean) (Override%20Tile%20Width? :type Boolean) (Override%20Tile%20Depth? :type Boolean) (Reverse%20Tile%20X? :type Boolean) (Reverse%20Tile%20Y? :type Boolean))
  (bind _returnvalue (AddComponent|AddHierarchicalInstancedStaticMeshComponent false))
  (Components|StaticMesh|SetStaticMesh _returnvalue Tile%20Mesh%2001)
  (for _index (range 0 (- (Variables|GeneralProperties|GetTileWidth) 1))
    (Components|InstancedStaticMesh|AddInstance _returnvalue (Math|Transform|MakeTransform (Math|Vector|MakeVector (+ X%20Offset (* _index (Math|Float|SelectFloat (* -1 (Math|Float|SelectFloat Override%20Tile%20Width (Math|Float|Absolute(Float) (Math|Float|SelectFloat (.x (.Min (Components|StaticMesh|GetLocalBounds _returnvalue))) (.x (.Max (Components|StaticMesh|GetLocalBounds _returnvalue))) UseMinXBound)) Override%20Tile%20Width?)) (Math|Float|SelectFloat Override%20Tile%20Width (Math|Float|Absolute(Float) (Math|Float|SelectFloat (.x (.Min (Components|StaticMesh|GetLocalBounds _returnvalue))) (.x (.Max (Components|StaticMesh|GetLocalBounds _returnvalue))) UseMinXBound)) Override%20Tile%20Width?) Reverse%20Tile%20X?))) Y%20Offset Z%20Offset) (Math|Rotator|MakeRotator 0.0 0.0 Rotation) "1.000000,1.000000,1.000000") false)
    (for _index_2 (range 1 (- (Variables|GeneralProperties|GetTileDepth) 1))
      (Components|InstancedStaticMesh|AddInstance _returnvalue (Math|Transform|MakeTransform (Math|Vector|MakeVector (+ X%20Offset (* _index (Math|Float|SelectFloat (* -1 (Math|Float|SelectFloat Override%20Tile%20Width (Math|Float|Absolute(Float) (Math|Float|SelectFloat (.x (.Min (Components|StaticMesh|GetLocalBounds _returnvalue))) (.x (.Max (Components|StaticMesh|GetLocalBounds _returnvalue))) UseMinXBound)) Override%20Tile%20Width?)) (Math|Float|SelectFloat Override%20Tile%20Width (Math|Float|Absolute(Float) (Math|Float|SelectFloat (.x (.Min (Components|StaticMesh|GetLocalBounds _returnvalue))) (.x (.Max (Components|StaticMesh|GetLocalBounds _returnvalue))) UseMinXBound)) Override%20Tile%20Width?) Reverse%20Tile%20X?))) (+ Y%20Offset (* _index_2 (Math|Float|SelectFloat (* -1 (Math|Float|SelectFloat Override%20Tile%20Depth (Math|Float|Absolute(Float) (Math|Float|SelectFloat (.y (.Min (Components|StaticMesh|GetLocalBounds _returnvalue))) (.y (.Max (Components|StaticMesh|GetLocalBounds _returnvalue))) UseMinYBound)) Override%20Tile%20Depth?)) (Math|Float|SelectFloat Override%20Tile%20Depth (Math|Float|Absolute(Float) (Math|Float|SelectFloat (.y (.Min (Components|StaticMesh|GetLocalBounds _returnvalue))) (.y (.Max (Components|StaticMesh|GetLocalBounds _returnvalue))) UseMinYBound)) Override%20Tile%20Depth?) Reverse%20Tile%20Y?))) Z%20Offset) (Math|Rotator|MakeRotator 0.0 0.0 Rotation) "1.000000,1.000000,1.000000") false))))