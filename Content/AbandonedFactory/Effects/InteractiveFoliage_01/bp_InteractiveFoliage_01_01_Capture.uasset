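; Scene capture actor that follows the player to feed an interactive foliage effect.
; On BeginPlay it sets the capture to show only components tagged InteractiveForce, capturing at about 60 FPS, and writes its ortho width to a material parameter collection.
; A looping timer, set when tagged components are found, moves it to the player's X/Y at fixed height and publishes that location to the same collection.
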(event EventBeginPlay
  (bind _interactivefoliagecapture (Variables|Default|GetInteractiveFoliageCapture))
  (Class|ActorComponent|SetComponentTickInterval _interactivefoliagecapture 0.016667) ; 60 FPS
  (Variables|/Script/Engine.SceneCaptureComponent|SetbCaptureEveryFrame _interactivefoliagecapture true)
  (Variables|/Script/Engine.SceneCaptureComponent|SetbCaptureOnMovement _interactivefoliagecapture true)
  (CallFunction|SetCaptureSize)
  (bind _outactors (Actor|GetAllActorswithTag "InteractiveForce"))
  (for _array_element _outactors
    (for _array_element_2 (Actor|GetComponentsbyTag _array_element "/Script/Engine.PrimitiveComponent" "InteractiveForce")
      (Rendering|SceneCapture|ShowOnlyComponent (Variables|Default|GetInteractiveFoliageCapture) _array_element_2)
      (Utilities|Time|SetTimerbyFunctionName self "MoveCapture" 0.016667 true) ; 60 FPS
    )))

(event EventTick
  (params (DeltaSeconds :type Float%20%28single-precision%29)))

(fn ConstructionScript)

(fn MoveCapture
  (bind _returnvalue (Game|GetPlayerCharacter 0))
  (bind _returnvalue_2 (Transformation|GetActorLocation _returnvalue))
  (Utilities|IsValid _returnvalue
    (:Is%20Valid
      (Transformation|SetActorLocation (Math|Vector|MakeVector (.x _returnvalue_2) (.y _returnvalue_2) (.z (Transformation|GetActorLocation))) false false)
      (Rendering|Material|SetVectorParameterValue "/Game/AbandonedFactory/Effects/InteractiveFoliage_01/mpc_InteractiveFoliage_01_01.mpc_InteractiveFoliage_01_01" "CaptureLocation" (Math|Conversions|ToLinearColor(Vector) (Transformation|GetActorLocation)) :!class /Script/Engine.KismetMaterialLibrary))))

(fn SetCaptureSize
  (Rendering|Material|SetScalarParameterValue "/Game/AbandonedFactory/Effects/InteractiveFoliage_01/mpc_InteractiveFoliage_01_01.mpc_InteractiveFoliage_01_01" "CaptureSize" (Variables|/Script/Engine.SceneCaptureComponent2D|GetOrthoWidth (Variables|Default|GetInteractiveFoliageCapture)) :!class /Script/Engine.KismetMaterialLibrary))